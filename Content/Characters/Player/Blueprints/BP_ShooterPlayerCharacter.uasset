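; Shooter player character Blueprint that adds the HUD widget on BeginPlay and defines a timeline-based directional dash.
; UseDashTimeline stores the X/Y input and restarts the dash timeline only when it is not already playing.
; The timeline's update logic projects the input direction onto the current floor plane, then applies a swept world offset scaled by the dash curve.
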(event EventBeginPlay
  (bind _returnvalue (UserInterface|CreateWidget "/Game/Blueprints/Widgets/BPW_PlayerHUD.BPW_PlayerHUD_C"))
  (UserInterface|Viewport|AddtoViewport _returnvalue 0))

(event Collision|EventActorBeginOverlap
  (params (OtherActor :type Actor%20Object%20Reference)))

(event EventTick
  (params (DeltaSeconds :type Float%20%28single-precision%29)))

(fn ConstructionScript)

(fn UseDashTimeline
  (params (InputX :type Float%20%28double-precision%29) (InputY :type Float%20%28double-precision%29))
  (bind _dashtimeline (Variables|Default|GetDashTimeline))
  (if (not (Audio|Components|Audio|IsPlaying _dashtimeline))
    (Variables|Default|SetInputX InputX)
    (Variables|Default|SetInputY InputY)
    (Components|Timeline|PlayfromStart _dashtimeline)))