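; Player controller for the shooter that maps Enhanced Input actions to movement, dash, aiming, shooting, pickups and item use.
; Equipped weapon data drives firing: chargeable weapons charge while held and fire on release, while others fire on trigger, then reset and reverse cached recoil on release.
; Weapons equip by slot key or scroll cycling through inventory slots.
; Grenade swapping is a temporary hardcoded frag/sticky toggle, and debug key J adds yaw.
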(event Input|EnhancedActionEvents|EnhancedInputActionIA_Jump
  (params (ActionValue :type Boolean) (ElapsedSeconds :type Float%20%28double-precision%29) (TriggeredSeconds :type Float%20%28double-precision%29) (InputAction :type Input%20Action%20Object%20Reference :default "/Game/Input/Actions/IA_Jump.IA_Jump"))
  (Class|ShooterPlayerController|Jump))

(event Input|EnhancedActionEvents|EnhancedInputActionIA_Dash
  (params (ActionValue :type Vector :default "0, 0, 0") (ElapsedSeconds :type Float%20%28double-precision%29) (TriggeredSeconds :type Float%20%28double-precision%29) (InputAction :type Input%20Action%20Object%20Reference :default "/Game/Input/Actions/IA_Dash.IA_Dash"))
  (if (and (> (.z ActionValue) 0.0) (<= (Variables|Default|GetDashCooldownValue) 0.0))
    (bind _asbp_shooter_player_character (Utilities|Casting|CastToBP_ShooterPlayerCharacter (Variables|Default|GetPlayerCharacter)))
    (Default|UseDashTimeline _asbp_shooter_player_character (.x ActionValue) (.y ActionValue))
    (Class|ShooterPlayerController|Dash)))

(event Input|EnhancedActionEvents|EnhancedInputActionIA_EquipPrimary
  (params (ActionValue :type Boolean) (ElapsedSeconds :type Float%20%28double-precision%29) (TriggeredSeconds :type Float%20%28double-precision%29) (InputAction :type Input%20Action%20Object%20Reference :default "/Game/Input/Actions/IA_EquipPrimary.IA_EquipPrimary"))
  (bind _playercharacter (Variables|Default|GetPlayerCharacter))
  ;[0 0.497 1] Equip Weapons
  (Class|ShooterPlayerCharacter|EquipWeapon _playercharacter (Variables|/Script/Gera_MovementShooter.InventoryComponent|GetPrimaryWeapon (Variables|/Script/Gera_MovementShooter.ShooterPlayerCharacter|GetInventoryComponent _playercharacter)))
  (Class|ShooterPlayerController|ResetWeapon))

(event Input|EnhancedActionEvents|EnhancedInputActionIA_EquipSecondary
  (params (ActionValue :type Boolean) (ElapsedSeconds :type Float%20%28double-precision%29) (TriggeredSeconds :type Float%20%28double-precision%29) (InputAction :type Input%20Action%20Object%20Reference :default "/Game/Input/Actions/IA_EquipSecondary.IA_EquipSecondary"))
  (bind _playercharacter (Variables|Default|GetPlayerCharacter))
  ;[0 0.497 1] Equip Weapons
  (Class|ShooterPlayerCharacter|EquipWeapon _playercharacter (Variables|/Script/Gera_MovementShooter.InventoryComponent|GetSecondaryWeapon (Variables|/Script/Gera_MovementShooter.ShooterPlayerCharacter|GetInventoryComponent _playercharacter)))
  (Class|ShooterPlayerController|ResetWeapon))

(event Input|EnhancedActionEvents|EnhancedInputActionIA_Shoot
  (params (ActionValue :type Boolean) (ElapsedSeconds :type Float%20%28double-precision%29) (TriggeredSeconds :type Float%20%28double-precision%29) (InputAction :type Input%20Action%20Object%20Reference :default "/Game/Input/Actions/IA_Shoot.IA_Shoot"))
  (bind _returnvalue (Class|ShooterPlayerController|GetEquippedWeaponData))
  (bind _returnvalue_2 (Class|ShooterPlayerController|GetEquippedWeaponData))
  (bind (_weaponslot _name _weapontype _weaponactor _staticmesh _outlinecolor _projectiletype _projectileactor _ammotype _ammocost _damage _firerate _zoommultiplier _aimingspreadoverride _aimingspreadindegrees _spreadindegrees _spreadmultiplier _hipfirerecoilminx _hipfirerecoilmaxx _hipfirerecoily _aimingrecoilminx _aimingrecoilmaxx _aimingrecoily _magazinecapacity _isshotgun _pelletcount _projectilevelocity _cancharge _minchargetime _maxchargetime) (Utilities|Struct|BreakWeaponData _returnvalue))
  (bind (_weaponslot_2 _name_2 _weapontype_2 _weaponactor_2 _staticmesh_2 _outlinecolor_2 _projectiletype_2 _projectileactor_2 _ammotype_2 _ammocost_2 _damage_2 _firerate_2 _zoommultiplier_2 _aimingspreadoverride_2 _aimingspreadindegrees_2 _spreadindegrees_2 _spreadmultiplier_2 _hipfirerecoilminx_2 _hipfirerecoilmaxx_2 _hipfirerecoily_2 _aimingrecoilminx_2 _aimingrecoilmaxx_2 _aimingrecoily_2 _magazinecapacity_2 _isshotgun_2 _pelletcount_2 _projectilevelocity_2 _cancharge_2) (Utilities|Struct|BreakWeaponData _returnvalue_2))
  ;[1 1 1] Shooting
  (:Triggered
    (switch Utilities|FlowControl|Switch|SwitchonEProjectileType _projectiletype
      (:Hitscan
        _)
      (:Projectile
        _))
    (if _cancharge
      (Class|ShooterPlayerController|ChargeShot _maxchargetime)
      (else
        (Class|ShooterPlayerController|Shoot false :!label _label))))
  (:Completed
    (switch Utilities|FlowControl|Switch|SwitchonEProjectileType _projectiletype_2
      (:None
        _)
      (:Hitscan
        (if _cancharge_2 :!label _label_2
          (goto _label)
          (else
            _)))
      (:Projectile
        (goto _label_2)))
    (Class|ShooterPlayerController|ResetWeapon)
    (Class|ShooterPlayerController|AddRecoil (Class|KismetMathLibrary|Negated2D (Variables|Default|GetRecoilCache)))))

(event Input|EnhancedActionEvents|EnhancedInputActionIA_CycleWeapons
  (params (ActionValue :type Float%20%28double-precision%29) (ElapsedSeconds :type Float%20%28double-precision%29) (TriggeredSeconds :type Float%20%28double-precision%29) (InputAction :type Input%20Action%20Object%20Reference :default "/Game/Input/Actions/IA_CycleWeapons.IA_CycleWeapons"))
  (bind _playercharacter (Variables|Default|GetPlayerCharacter))
  (bind _inventorycomponent (Variables|/Script/Gera_MovementShooter.ShooterPlayerCharacter|GetInventoryComponent _playercharacter))
  (bind _equippedweapon (Variables|/Script/Gera_MovementShooter.ShooterPlayerCharacter|GetEquippedWeapon _playercharacter))
  (bind (_datatable _rowname) (Utilities|Struct|BreakDataTableRowHandle _equippedweapon))
  ;[0.4247 0 1] Cycle Weapons with Scroll Wheel
  (bind _returnvalue (Utilities|GetDataTableRow _datatable _rowname)
    (:then
      (if (> ActionValue 0.0)
        (switch Utilities|FlowControl|Switch|SwitchonEWeaponSlot (.WeaponSlot (Utilities|Struct|BreakWeaponData _returnvalue))
          (:Primary
            (Class|ShooterPlayerCharacter|EquipWeapon _playercharacter (Variables|/Script/Gera_MovementShooter.InventoryComponent|GetSecondaryWeapon _inventorycomponent)))
          (:Secondary
            (Class|ShooterPlayerCharacter|EquipWeapon _playercharacter (Variables|/Script/Gera_MovementShooter.InventoryComponent|GetHeavyWeapon _inventorycomponent)))
          (:Heavy
            (Class|ShooterPlayerCharacter|EquipWeapon _playercharacter (Variables|/Script/Gera_MovementShooter.InventoryComponent|GetPrimaryWeapon _inventorycomponent))))
        (elif (< ActionValue 0.0)
          (switch Utilities|FlowControl|Switch|SwitchonEWeaponSlot (.WeaponSlot (Utilities|Struct|BreakWeaponData _returnvalue))
            (:Primary
              (Class|ShooterPlayerCharacter|EquipWeapon _playercharacter (Variables|/Script/Gera_MovementShooter.InventoryComponent|GetHeavyWeapon _inventorycomponent)))
            (:Secondary
              (Class|ShooterPlayerCharacter|EquipWeapon _playercharacter (Variables|/Script/Gera_MovementShooter.InventoryComponent|GetPrimaryWeapon _inventorycomponent)))
            (:Heavy
              (Class|ShooterPlayerCharacter|EquipWeapon _playercharacter (Variables|/Script/Gera_MovementShooter.InventoryComponent|GetSecondaryWeapon _inventorycomponent)))))))))

(event Input|EnhancedActionEvents|EnhancedInputActionIA_EquipHeavy
  (params (ActionValue :type Boolean) (ElapsedSeconds :type Float%20%28double-precision%29) (TriggeredSeconds :type Float%20%28double-precision%29) (InputAction :type Input%20Action%20Object%20Reference :default "/Game/Input/Actions/IA_EquipHeavy.IA_EquipHeavy"))
  (bind _playercharacter (Variables|Default|GetPlayerCharacter))
  ;[0 0.497 1] Equip Weapons
  (Class|ShooterPlayerCharacter|EquipWeapon _playercharacter (Variables|/Script/Gera_MovementShooter.InventoryComponent|GetHeavyWeapon (Variables|/Script/Gera_MovementShooter.ShooterPlayerCharacter|GetInventoryComponent _playercharacter)))
  (Class|ShooterPlayerController|ResetWeapon))

(event Input|EnhancedActionEvents|EnhancedInputActionIA_UseSupportItem
  (params (ActionValue :type Boolean) (ElapsedSeconds :type Float%20%28double-precision%29) (TriggeredSeconds :type Float%20%28double-precision%29) (InputAction :type Input%20Action%20Object%20Reference :default "/Game/Input/Actions/IA_UseSupportItem.IA_UseSupportItem"))
  (Class|ShooterPlayerController|UseBuffItem))

(event Input|EnhancedActionEvents|EnhancedInputActionIA_Crouch
  (params (ActionValue :type Boolean) (ElapsedSeconds :type Float%20%28double-precision%29) (TriggeredSeconds :type Float%20%28double-precision%29) (InputAction :type Input%20Action%20Object%20Reference :default "/Game/Input/Actions/IA_Crouch.IA_Crouch"))
  (:Triggered
    (Class|ShooterPlayerController|Crouch))
  (:Completed
    (Class|ShooterPlayerController|StopCrouch)))

(event Input|EnhancedActionEvents|EnhancedInputActionIA_UseThrowableItem
  (params (ActionValue :type Boolean) (ElapsedSeconds :type Float%20%28double-precision%29) (TriggeredSeconds :type Float%20%28double-precision%29) (InputAction :type Input%20Action%20Object%20Reference :default "/Game/Input/Actions/IA_UseThrowableItem.IA_UseThrowableItem"))
  (Class|ShooterPlayerController|UseThrowableItem))

(event Input|EnhancedActionEvents|EnhancedInputActionIA_SwapGrenade
  (params (ActionValue :type Boolean) (ElapsedSeconds :type Float%20%28double-precision%29) (TriggeredSeconds :type Float%20%28double-precision%29) (InputAction :type Input%20Action%20Object%20Reference :default "/Game/Input/Actions/IA_SwapGrenade.IA_SwapGrenade"))
  ;[1 0 0] Cycle Between Throwables (VERY TEMPORARY... FIX LATER!!!)
  (if (== (.Name (Utilities|Struct|BreakItemData (Class|InventoryComponent|GetEquippedEquipmentData (Variables|/Script/Gera_MovementShooter.ShooterPlayerCharacter|GetInventoryComponent (Variables|Default|GetPlayerCharacter))))) "Frag Grenade")
    (Class|InventoryComponent|SwapEquipment (Variables|/Script/Gera_MovementShooter.ShooterPlayerCharacter|GetInventoryComponent (Variables|Default|GetPlayerCharacter)) (Utilities|Struct|MakeDataTableRowHandle "/Game/DataTables/DT_Items.DT_Items" "StickyGrenade"))
    (else
      (Class|InventoryComponent|SwapEquipment (Variables|/Script/Gera_MovementShooter.ShooterPlayerCharacter|GetInventoryComponent (Variables|Default|GetPlayerCharacter)) (Utilities|Struct|MakeDataTableRowHandle "/Game/DataTables/DT_Items.DT_Items" "FragGrenade")))))

(event Input|EnhancedActionEvents|EnhancedInputActionIA_Look
  (params (ActionValue :type Vector%202D%20Structure) (ElapsedSeconds :type Float%20%28double-precision%29) (TriggeredSeconds :type Float%20%28double-precision%29) (InputAction :type Input%20Action%20Object%20Reference :default "/Game/Input/Actions/IA_Look.IA_Look"))
  (Class|ShooterPlayerController|AddLookInput ActionValue))

(event Input|EnhancedActionEvents|EnhancedInputActionIA_Move
  (params (ActionValue :type Vector%202D%20Structure) (ElapsedSeconds :type Float%20%28double-precision%29) (TriggeredSeconds :type Float%20%28double-precision%29) (InputAction :type Input%20Action%20Object%20Reference :default "/Game/Input/Actions/IA_Move.IA_Move"))
  (Class|ShooterPlayerController|Move (.x ActionValue) (.y ActionValue)))

(event Input|EnhancedActionEvents|EnhancedInputActionIA_PickupItem
  (params (ActionValue :type Boolean) (ElapsedSeconds :type Float%20%28double-precision%29) (TriggeredSeconds :type Float%20%28double-precision%29) (InputAction :type Input%20Action%20Object%20Reference :default "/Game/Input/Actions/IA_PickupItem.IA_PickupItem"))
  (Class|ShooterPlayerCharacter|PickupItem (Variables|Default|GetPlayerCharacter))
  (bind _foundwidgets (Widget|GetAllWidgetsOfClass "/Game/Blueprints/Widgets/BPW_PlayerHUD.BPW_PlayerHUD_C" true))
  (for _array_element _foundwidgets
    (Variables|/Game/Blueprints/Widgets/BPW_PlayerHUD.BPW_PlayerHUD_C|SetPickupItemName _array_element "None")))

(event Input|EnhancedActionEvents|EnhancedInputActionIA_Aim
  (params (ActionValue :type Boolean) (ElapsedSeconds :type Float%20%28double-precision%29) (TriggeredSeconds :type Float%20%28double-precision%29) (InputAction :type Input%20Action%20Object%20Reference :default "/Game/Input/Actions/IA_Aim.IA_Aim"))
  (:Triggered
    (Class|ShooterPlayerController|Aim (.ZoomMultiplier (Utilities|Struct|BreakWeaponData (Class|ShooterPlayerController|GetEquippedWeaponData)))))
  (:Completed
    (Class|ShooterPlayerController|StopAiming)))

(event EventBeginPlay
  (Class|PlayerController|SetDeprecatedInputYawScale 1.0)
  (Class|PlayerController|SetDeprecatedInputPitchScale 1.0))

(event Input|KeyboardEvents|DebugKeyJ
  (params (Key :type Key%20Structure :default "None") (ActionValue :type Input%20Action%20Value%20Structure))
  (:Pressed
    (Class|PlayerController|AddYawInput 9e+01)))

(fn ConstructionScript)