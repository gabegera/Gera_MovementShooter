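; AI controller for the Shotgunner enemy, a ranged enemy driven by the BT_ShotgunnerEnemy behavior tree.
; On BeginPlay it starts the tree and sets the IsArmed blackboard key based on whether the character's weapon child actor is valid.
; Perception updates for the player pawn write the sensing result to CanSeeTarget, feeding sight state to the tree.
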(event OnTargetPerceptionUpdated(PerceptionComponent)
  (params (Actor :type Actor%20Object%20Reference) (Stimulus :type AI%20Stimulus%20Structure))
  (if (== Actor (Game|Player|GetPlayerPawn 0))
    (AI|Components|Blackboard|SetValueasBool (AI|GetBlackboard 0) (Utilities|Name|MakeLiteralName "CanSeeTarget") (.bsuccessfullysensed Stimulus))))

(event EventBeginPlay
  (AI|RunBehaviorTree "/Game/Characters/Enemies/AI/BehaviorTree/BT_ShotgunnerEnemy.BT_ShotgunnerEnemy")
  (AI|Components|Blackboard|SetValueasBool (AI|GetBlackboard 0) (Utilities|Name|MakeLiteralName "IsArmed") (Utilities|IsValid (Variables|/Script/Engine.ChildActorComponent|GetChildActor (Variables|/Script/Gera_MovementShooter.ShooterCharacter|GetWeaponChildComponent (Class|BaseEnemyAIController|GetEnemyCharacter))))))

(fn ConstructionScript)