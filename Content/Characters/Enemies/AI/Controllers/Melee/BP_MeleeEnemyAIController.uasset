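; AI controller for melee enemies that drives them with the BT_MeleeEnemy behavior tree.
; On BeginPlay it runs the tree and seeds the blackboard with the first player's pawn as Target and its position as TargetLocation.
; It sets CanAttack by comparing the player-to-enemy distance against MeleeAttackDistance.
; These keys are written only once at startup and are not refreshed by this controller.
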(event EventBeginPlay
  (bind _returnvalue (Game|Player|GetPlayerPawn 0))
  (bind _returnvalue_2 (AI|GetBlackboard 0))
  (bind _returnvalue_3 (Transformation|GetActorLocation _returnvalue))
  (AI|RunBehaviorTree "/Game/Characters/Enemies/AI/BehaviorTree/BT_MeleeEnemy.BT_MeleeEnemy")
  (AI|Components|Blackboard|SetValueasObject _returnvalue_2 (Utilities|Name|MakeLiteralName "Target") _returnvalue)
  (AI|Components|Blackboard|SetValueasVector _returnvalue_2 (Utilities|Name|MakeLiteralName "TargetLocation") _returnvalue_3)
  (AI|Components|Blackboard|SetValueasBool _returnvalue_2 (Utilities|Name|MakeLiteralName "CanAttack") (<= (Math|Vector|Distance(Vector) _returnvalue_3 (Transformation|GetActorLocation (Class|BaseEnemyAIController|GetEnemyCharacter))) (Variables|Default|GetMeleeAttackDistance))))

(fn ConstructionScript)