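; Enemy AI controller that runs a melee or ranged behavior tree according to the enemy type.
; On BeginPlay it also writes the player pawn, its location and a CanAttack flag from the melee attack distance to the Blackboard, with no later refresh of these values.
; Perception updates for the player pawn set CanSeeTarget from whether the stimulus was sensed.
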(event OnTargetPerceptionUpdated(PerceptionComponent)
  (params (Actor :type Actor%20Object%20Reference) (Stimulus :type AI%20Stimulus%20Structure))
  (if (== Actor (Game|Player|GetPlayerPawn 0))
    (AI|Components|Blackboard|SetValueasBool (AI|GetBlackboard 0) (Utilities|Name|MakeLiteralName "CanSeeTarget") (.bsuccessfullysensed Stimulus))))

(event EventBeginPlay
  (bind _returnvalue (Game|Player|GetPlayerPawn 0))
  (bind _returnvalue_2 (AI|GetBlackboard 0))
  (bind _returnvalue_3 (Transformation|GetActorLocation _returnvalue))
  (switch Utilities|FlowControl|Switch|SwitchonEEnemyType (Class|BaseEnemyAIController|GetEnemyType)
    (:Melee
      (AI|RunBehaviorTree "/Game/Characters/Enemies/AI/BehaviorTree/BT_MeleeEnemy.BT_MeleeEnemy"))
    (:Ranged
      (AI|RunBehaviorTree "/Game/Characters/Enemies/AI/BehaviorTree/BT_RangedEnemy.BT_RangedEnemy")))
  (AI|Components|Blackboard|SetValueasObject _returnvalue_2 (Utilities|Name|MakeLiteralName "Target") _returnvalue)
  (AI|Components|Blackboard|SetValueasVector _returnvalue_2 (Utilities|Name|MakeLiteralName "TargetLocation") _returnvalue_3)
  (AI|Components|Blackboard|SetValueasBool _returnvalue_2 (Utilities|Name|MakeLiteralName "CanAttack") (<= (Math|Vector|Distance(Vector) _returnvalue_3 (Transformation|GetActorLocation (Class|BaseEnemyAIController|GetEnemyCharacter))) (Variables|Default|GetMeleeAttackDistance))))

(fn ConstructionScript)