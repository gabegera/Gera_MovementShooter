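; Thrown frag grenade, marked OLD by its file name, that explodes on a fuse timer and damages its surroundings.
; On BeginPlay it reads blast radius and damage from the player 0 inventory equipment slot's data table row, then starts the fuse.
; The explosion applies radial damage with equal inner and outer radii, credited to player 0, draws a debug sphere trace and destroys the actor.
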(event Custom|Explode
  (bind _returnvalue (Transformation|GetActorLocation))
  (bind _blastradius (Variables|Default|GetBlastRadius))
  (Class|GameplayStatics|ApplyRadialDamagewithFalloff (Variables|Default|GetDamage) 0.0 _returnvalue _blastradius _blastradius 0.0 "/Script/Engine.DamageType" 0 self (Pawn|GetController (Game|GetPlayerCharacter 0)) "ECC_Visibility")
  ;[1 1 1] Debug Draw Sphere Trace
  (Collision|MultiSphereTraceForObjects _returnvalue _returnvalue _blastradius (Utilities|Array|MakeArray "ObjectTypeQuery3") false 0 "ForDuration" true "(R=1.000000,G=0.000000,B=0.000000,A=1.000000)" "(R=0.000000,G=1.000000,B=0.000000,A=1.000000)" 1.0)
  (Actor|DestroyActor))

(event EventBeginPlay
  (bind _returnvalue (Game|Player|GetPlayerPawn 0))
  (bind _returnvalue_2 (Actor|GetComponentbyClass _returnvalue "/Script/Gera_MovementShooter.InventoryComponent"))
  (bind _equipmentslot (Variables|/Script/Gera_MovementShooter.InventoryComponent|GetEquipmentSlot _returnvalue_2))
  (bind (_datatable _rowname) (Utilities|Struct|BreakDataTableRowHandle _equipmentslot))
  (bind _returnvalue_3 (Utilities|GetDataTableRow _datatable _rowname)
    (:then
      (Variables|Default|SetBlastRadius (.BlastRadius (Utilities|Struct|BreakEquipmentData _returnvalue_3)))
      (Variables|Default|SetDamage (.Damage (Utilities|Struct|BreakEquipmentData _returnvalue_3)))
      (Utilities|Time|SetTimerbyEvent (delegate Custom|Explode) (Variables|Default|GetFuseTime)))))

(fn ConstructionScript)