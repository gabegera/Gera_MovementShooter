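; Grenade projectile that damages what it hits, can knock physics props away, and destroys itself on impact.
; BeginPlay caches the first BP_ShooterPlayerCharacter found in the world, and Hit passes it, its controller and the hit actor to DealDamage, which is defined outside these graphs.
; If the hit actor's static mesh simulates physics, it alone receives a mass-independent radial impulse with constant falloff.
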(event Collision|EventHit
  (params (MyComp :type Primitive%20Component%20Object%20Reference) (Other :type Actor%20Object%20Reference) (OtherComp :type Primitive%20Component%20Object%20Reference) (bSelfMoved :type Boolean) (HitLocation :type Vector :default "0, 0, 0") (HitNormal :type Vector :default "0, 0, 0") (NormalImpulse :type Vector :default "0, 0, 0") (Hit :type Hit%20Result%20Structure%20%28by%20ref%29))
  (bind _returnvalue (Actor|GetComponentbyClass Other "/Script/Engine.StaticMeshComponent"))
  (bind _playercharacter (Variables|Default|GetPlayerCharacter))
  (bind _asbp_shooter_player_character (Utilities|Casting|CastToBP_ShooterPlayerCharacter _playercharacter)
    (:then
      (Class|GrenadeProjectile|DealDamage Other _asbp_shooter_player_character (Pawn|GetController _playercharacter))
      (Utilities|IsValid _returnvalue
        (:Is%20Valid
          (if (Physics|IsSimulatingPhysics _returnvalue "None")
            (Physics|AddRadialImpulse _returnvalue "0, 0, 0" 2048.0 1e+03 "RIF_Constant" true)
            (Actor|DestroyActor)
            (else
              (Actor|DestroyActor :!label _label))))
        (:Is%20Not%20Valid
          (goto _label))))
    (:CastFailed
      (Actor|DestroyActor))))

(event EventBeginPlay
  (bind _returnvalue (Actor|GetActorOfClass "/Game/Blueprints/Player/BP_ShooterPlayerCharacter.BP_ShooterPlayerCharacter_C"))
  (Variables|Default|SetPlayerCharacter _returnvalue))

(fn ConstructionScript)