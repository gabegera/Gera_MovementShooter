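; AI controller for enemies that starts a melee or ranged behavior tree based on the enemy type.
; On BeginPlay it runs the matching tree, then seeds the blackboard with the player pawn as Target, its location and a CanAttack flag.
; CanAttack compares player distance to MeleeAttackDistance for both types.
; These values are written only once, as Tick is empty.
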(event EventBeginPlay
  (bind _returnvalue (Game|Player|GetPlayerPawn 0))
  (bind _returnvalue_2 (AI|GetBlackboard 0))
  (bind _returnvalue_3 (Transformation|GetActorLocation _returnvalue))
  (switch Utilities|FlowControl|Switch|SwitchonEEnemyType (Class|EnemyAIController|GetEnemyType)
    (:Melee
      (AI|RunBehaviorTree "/Game/Blueprints/Enemies/AI/BehaviorTree/BT_MeleeEnemy.BT_MeleeEnemy"))
    (:Ranged
      (AI|RunBehaviorTree "/Game/Blueprints/Enemies/AI/BehaviorTree/BT_RangedEnemy.BT_RangedEnemy")))
  (AI|Components|Blackboard|SetValueasObject _returnvalue_2 (Utilities|Name|MakeLiteralName "Target") _returnvalue)
  (AI|Components|Blackboard|SetValueasVector _returnvalue_2 (Utilities|Name|MakeLiteralName "TargetLocation") _returnvalue_3)
  (AI|Components|Blackboard|SetValueasBool _returnvalue_2 (Utilities|Name|MakeLiteralName "CanAttack") (<= (Math|Vector|Distance(Vector) _returnvalue_3 (Transformation|GetActorLocation (Class|EnemyAIController|GetEnemyCharacter))) (Variables|Default|GetMeleeAttackDistance))))

(event EventTick
  (params (DeltaSeconds :type Float%20%28single-precision%29)))

(fn ConstructionScript)