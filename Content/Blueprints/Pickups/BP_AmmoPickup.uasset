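; Ammo pickup actor that grants ammo to the player on touch.
; BeginPlay caches the first BP_ShooterPlayerCharacter found, and the sphere collision overlap responds only to that actor.
; It switches on a weapon-type variable named RIFLE to pass the rifle, shotgun or grenade launcher amount to the player controller's AddAmmo, then destroys itself.
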(event OnComponentBeginOverlap(SphereCollision)
  (params (OverlappedComponent :type Primitive%20Component%20Object%20Reference) (OtherActor :type Actor%20Object%20Reference) (OtherComp :type Primitive%20Component%20Object%20Reference) (OtherBodyIndex :type Integer) (bFromSweep :type Boolean) (SweepResult :type Hit%20Result%20Structure%20%28by%20ref%29))
  (if (== OtherActor (Variables|Default|GetPlayerCharacter))
    (bind _asbp_shooter_player_controller (Utilities|Casting|CastToBP_ShooterPlayerController (Pawn|GetController (Variables|Default|GetPlayerCharacter))))
    (switch Utilities|FlowControl|Switch|SwitchonAmmoType "RIFLE"
      (:RIFLE
        (Class|ShooterPlayerController|AddAmmo _asbp_shooter_player_controller (Variables|Default|GetRifleAmmo)))
      (:SHOTGUN
        (Class|ShooterPlayerController|AddAmmo _asbp_shooter_player_controller (Variables|Default|GetShotgunAmmo)))
      (:GRENADELAUNCHER
        (Class|ShooterPlayerController|AddAmmo _asbp_shooter_player_controller (Variables|Default|GetGrenadeLauncherAmmo))))
    (Actor|DestroyActor)))

(event EventBeginPlay
  (bind _returnvalue (Actor|GetActorOfClass "/Game/Blueprints/Player/BP_ShooterPlayerCharacter.BP_ShooterPlayerCharacter_C"))
  (Variables|Default|SetPlayerCharacter _returnvalue))

(event Collision|EventActorBeginOverlap
  (params (OtherActor :type Actor%20Object%20Reference)))

(event EventTick
  (params (DeltaSeconds :type Float%20%28single-precision%29)))

(fn ConstructionScript)